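; Pickup actor that the player collects by interacting while in its collision volume and empty-handed.
; Overlap toggles the interact widget and a Tick check of the character's interact and held-item state.
; A one-shot Delay loop counts Timer down with walk speed zeroed, then restores speed, destroys the actor and sets itself as ItemHolding.
; The failed check prints "Already Holding Item" once, even when simply not interacting.
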(event OnComponentBeginOverlap(collision)
  (params (OverlappedComponent :type Primitive%20Component%20Object%20Reference) (OtherActor :type Actor%20Object%20Reference) (OtherComp :type Primitive%20Component%20Object%20Reference) (OtherBodyIndex :type Integer) (bFromSweep :type Boolean) (SweepResult :type Hit%20Result%20Structure%20%28by%20ref%29))
  (bind (_asfirst_person_character_thijs _bsuccess) (Utilities|Casting|CastToFirstPersonCharacter_THIJS OtherActor))
  (if _bsuccess
    (Variables|Default|SetStartChecking true)
    (UserInterface|Viewport|AddtoViewport (Variables|/Game/_GAME/Blueprints/FirstPersonBP/Blueprints/FirstPersonCharacter_THIJS.FirstPersonCharacter_THIJS_C|GetInteractWidget _asfirst_person_character_thijs) 0)))

(event OnComponentEndOverlap(collision)
  (params (OverlappedComponent :type Primitive%20Component%20Object%20Reference) (OtherActor :type Actor%20Object%20Reference) (OtherComp :type Primitive%20Component%20Object%20Reference) (OtherBodyIndex :type Integer))
  (bind (_asfirst_person_character_thijs _bsuccess) (Utilities|Casting|CastToFirstPersonCharacter_THIJS OtherActor))
  (if _bsuccess
    (Variables|Default|SetStartChecking false)
    (Widget|RemovefromParent (Variables|/Game/_GAME/Blueprints/FirstPersonBP/Blueprints/FirstPersonCharacter_THIJS.FirstPersonCharacter_THIJS_C|GetInteractWidget _asfirst_person_character_thijs))))

(event EventBeginPlay
  (Components|StaticMesh|SetStaticMesh (Variables|Default|GetStaticMesh) (Variables|Default|GetStatic%20Mesh)))

(event EventTick
  (params (DeltaSeconds :type Float%20%28single-precision%29))
  (if (Variables|Default|GetStartChecking)
    (bind _asfirst_person_character_thijs (Utilities|Casting|CastToFirstPersonCharacter_THIJS (Game|GetPlayerCharacter 0)))
    (if (and (Variables|/Game/_GAME/Blueprints/FirstPersonBP/Blueprints/FirstPersonCharacter_THIJS.FirstPersonCharacter_THIJS_C|GetIsInteracting _asfirst_person_character_thijs) (== (Variables|/Game/_GAME/Blueprints/FirstPersonBP/Blueprints/FirstPersonCharacter_THIJS.FirstPersonCharacter_THIJS_C|GetItemHolding _asfirst_person_character_thijs) 0))
      (Utilities|FlowControl|DoOnce false
        (:Completed
          (Utilities|FlowControl|Delay 0.1 :!label _label)
          (Variables|/Script/Engine.CharacterMovementComponent|SetMaxWalkSpeed (Variables|/Script/Engine.Character|GetCharacterMovement _asfirst_person_character_thijs) 0.0)
          (bind _output_get (Variables|Default|SetTimer (- (Variables|Default|GetTimer) 0.1)))
          (Development|PrintString (Utilities|String|ToString(Float) _output_get))
          (if (<= (Variables|Default|GetTimer) 0.0)
            (Variables|/Script/Engine.CharacterMovementComponent|SetMaxWalkSpeed (Variables|/Script/Engine.Character|GetCharacterMovement _asfirst_person_character_thijs) 4e+02)
            (Development|PrintString "Picked Up Item")
            (Actor|DestroyActor)
            (bind _asfirst_person_character_thijs_2 (Utilities|Casting|CastToFirstPersonCharacter_THIJS (Game|GetPlayerCharacter 0)))
            (Variables|/Game/_GAME/Blueprints/FirstPersonBP/Blueprints/FirstPersonCharacter_THIJS.FirstPersonCharacter_THIJS_C|SetItemHolding _asfirst_person_character_thijs_2 self)
            (else
              (goto _label)))))
      (else
        (Utilities|FlowControl|DoOnce false
          (:Completed
            (Development|PrintString "Already Holding Item")))))))

(fn ConstructionScript)