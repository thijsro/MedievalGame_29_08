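; Delivery point where a player carrying an item hands it in, counting toward the Knights' win.
; Sphere overlap toggles the character's interact widget and a Tick check for interacting while holding an item.
; A DoOnce, reset on leaving the sphere, clears the held item and increments ItemsSaved on MainGameMode.
; When that count equals the TotalPickups length, it calls KnightsWIN.
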(event OnComponentBeginOverlap(Sphere)
  (params (OverlappedComponent :type Primitive%20Component%20Object%20Reference) (OtherActor :type Actor%20Object%20Reference) (OtherComp :type Primitive%20Component%20Object%20Reference) (OtherBodyIndex :type Integer) (bFromSweep :type Boolean) (SweepResult :type Hit%20Result%20Structure%20%28by%20ref%29))
  (bind (_asfirst_person_character_thijs _bsuccess) (Utilities|Casting|CastToFirstPersonCharacter_THIJS OtherActor))
  (if _bsuccess
    (Variables|Default|SetStartChecking true)
    (UserInterface|Viewport|AddtoViewport (Variables|/Game/_GAME/Blueprints/FirstPersonBP/Blueprints/FirstPersonCharacter_THIJS.FirstPersonCharacter_THIJS_C|GetInteractWidget _asfirst_person_character_thijs) 0)))

(event OnComponentEndOverlap(Sphere)
  (params (OverlappedComponent :type Primitive%20Component%20Object%20Reference) (OtherActor :type Actor%20Object%20Reference) (OtherComp :type Primitive%20Component%20Object%20Reference) (OtherBodyIndex :type Integer))
  (bind (_asfirst_person_character_thijs _bsuccess) (Utilities|Casting|CastToFirstPersonCharacter_THIJS OtherActor))
  (if _bsuccess
    (Variables|Default|SetStartChecking false)
    (Widget|RemovefromParent (Variables|/Game/_GAME/Blueprints/FirstPersonBP/Blueprints/FirstPersonCharacter_THIJS.FirstPersonCharacter_THIJS_C|GetInteractWidget _asfirst_person_character_thijs))
    (Utilities|FlowControl|DoOnce false) ; enters at Reset
  ))

(event EventBeginPlay)

(event Collision|EventActorBeginOverlap
  (params (OtherActor :type Actor%20Object%20Reference)))

(event EventTick
  (params (DeltaSeconds :type Float%20%28single-precision%29))
  (if (Variables|Default|GetStartChecking)
    (bind _asfirst_person_character_thijs (Utilities|Casting|CastToFirstPersonCharacter_THIJS (Game|GetPlayerCharacter 0)))
    (if (and (Variables|/Game/_GAME/Blueprints/FirstPersonBP/Blueprints/FirstPersonCharacter_THIJS.FirstPersonCharacter_THIJS_C|GetIsInteracting _asfirst_person_character_thijs) (!= (Variables|/Game/_GAME/Blueprints/FirstPersonBP/Blueprints/FirstPersonCharacter_THIJS.FirstPersonCharacter_THIJS_C|GetItemHolding _asfirst_person_character_thijs) 0))
      (Utilities|FlowControl|DoOnce false
        (:Completed
          (Variables|/Game/_GAME/Blueprints/FirstPersonBP/Blueprints/FirstPersonCharacter_THIJS.FirstPersonCharacter_THIJS_C|SetItemHolding _asfirst_person_character_thijs 0)
          (bind _asmain_game_mode (Utilities|Casting|CastToMainGameMode (Game|GetGameMode)))
          (bind _output_get (Variables|/Game/_GAME/MainGameMode.MainGameMode_C|SetItemsSaved _asmain_game_mode (+ (Variables|/Game/_GAME/MainGameMode.MainGameMode_C|GetItemsSaved _asmain_game_mode) 1)))
          (Development|PrintString (Utilities|String|ToString(Integer) _output_get))
          (if (== (Variables|/Game/_GAME/MainGameMode.MainGameMode_C|GetItemsSaved _asmain_game_mode) (Utilities|Array|Length (Variables|/Game/_GAME/MainGameMode.MainGameMode_C|GetTotalPickups _asmain_game_mode)))
            (Default|KnightsWIN _asmain_game_mode)))))))

(fn ConstructionScript)