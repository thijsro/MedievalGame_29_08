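; CastleGate_BP is a castle gate actor that rises vertically when opened.
; BeginPlay stores the starting world location and derives a goal raised on Z by AddedHeight.
; The GateOpen event plays a timeline from the start, lerping between the two positions and applying the result as relative location.
; The file contains no closing logic and no caller for GateOpen.
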(event Custom|GateOpen
  (bind _progress (Timeline|OpenGateTimeline PlayFromStart)
    (:Update
      (Transformation|SetActorRelativeLocation self (Math|Vector|Lerp(Vector) (Variables|Default|GetStartLocation) (Variables|Default|GetGoalLocation) _progress)))))

(event EventBeginPlay
  (bind _output_get (Variables|Default|SetStartLocation (Transformation|GetActorLocation self)))
  (Variables|Default|SetGoalLocation (+ "0, 0, 0" (Math|Vector|MakeVector (.x _output_get) (.y _output_get) (+ (.z _output_get) (Variables|Default|GetAddedHeight))))))

(fn ConstructionScript)